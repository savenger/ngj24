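; End-of-match actor that decides a two-player sheep-collecting car game when the timer runs out.
; On BeginPlay it finds the TimerManager and binds to its timer-over event.
; On expiry it finds the car pawn with the most collected sheep, flips that player index to the loser's, and passes it to OpenEndGamePanel.
; A debug helper that forces a winner and an unfinished equal-score check are left unwired.
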(event Custom|OnTimerExpired
  (bind _outactors (Actor|GetAllActorsOfClass "/Game/VehicleTemplate/Blueprints/OffroadCar/BP_OffroadCar_Pawn.BP_OffroadCar_Pawn_C"))
  (for _array_element _outactors
    (Utilities|Array|Add (Variables|Default|GetSheepCollectedIntArray) (Variables|/Game/VehicleTemplate/Blueprints/OffroadCar/BP_OffroadCar_Pawn.BP_OffroadCar_Pawn_C|GetCollected _array_element))
    (if (> (Variables|/Game/VehicleTemplate/Blueprints/OffroadCar/BP_OffroadCar_Pawn.BP_OffroadCar_Pawn_C|GetCollected _array_element) (Variables|Default|GetMaxSheepCollected))
      (Variables|Default|SetMaxSheepCollected (Variables|/Game/VehicleTemplate/Blueprints/OffroadCar/BP_OffroadCar_Pawn.BP_OffroadCar_Pawn_C|GetCollected _array_element))
      (Variables|Default|SetPlayerIndexWIthMoreSheep (Variables|/Script/CarSample.CarSampleOffroadCar|GetCarOffroadPlayerIndex _array_element))
      (Development|PrintString (Utilities|String|BuildString(Integer) "Player with more shee is " "with  n " (Variables|/Script/CarSample.CarSampleOffroadCar|GetCarOffroadPlayerIndex _array_element)))
      (Development|PrintString (Utilities|String|ToString(Integer) (Variables|/Game/VehicleTemplate/Blueprints/OffroadCar/BP_OffroadCar_Pawn.BP_OffroadCar_Pawn_C|GetCollected _array_element)))))
  ;[1 1 1] We have the winner index, so we calculate the looser one
  (if (== (Variables|Default|GetPlayerIndexWIthMoreSheep) 0)
    (Variables|Default|SetPlayerIndexWIthMoreSheep 1)
    (else
      (Variables|Default|SetPlayerIndexWIthMoreSheep 0)))
  (Class|EndGameActor|OpenEndGamePanel (Variables|Default|GetPlayerIndexWIthMoreSheep)))

(event EventBeginPlay
  (Utilities|FlowControl|Sequence
    (:then_0
      (Variables|Default|SetPlayerIndexWIthMoreSheep 0)
      (Variables|Default|SetMaxSheepCollected 0))
    (:then_1
      (bind _returnvalue (Actor|GetActorOfClass "/Game/UI/TimerManager.TimerManager_C"))
      (Utilities|IsValid _returnvalue
        (:Is%20Valid
          (bind _output_get (Variables|Default|SetTimerManagers _returnvalue))
          (EventDispatchers|BindEventtoOnTimerOver _output_get (delegate Custom|OnTimerExpired)))))))

(event Collision|EventActorBeginOverlap
  (params (OtherActor :type Actor%20Object%20Reference)))

(event EventTick
  (params (DeltaSeconds :type Float%20%28single-precision%29)))

(fn ConstructionScript)

(fn DebugSheepCollectedWinner
  (params (WinnerPlayerIndex :type Integer))
  (LocalVariables|SetDebugWinnerPlayerIndex WinnerPlayerIndex)
  (bind _outactors (Actor|GetAllActorsOfClass "/Game/VehicleTemplate/Blueprints/OffroadCar/BP_OffroadCar_Pawn.BP_OffroadCar_Pawn_C"))
  (bind _array_element (Utilities|Array|ForEachLoopwithBreak _outactors :!label _label)
    (:LoopBody
      (if (== (Variables|/Script/CarSample.CarSampleOffroadCar|GetCarOffroadPlayerIndex _array_element) (LocalVariables|GetDebugWinnerPlayerIndex))
        (Variables|/Game/VehicleTemplate/Blueprints/OffroadCar/BP_OffroadCar_Pawn.BP_OffroadCar_Pawn_C|SetCollected _array_element 50)
        (Development|PrintString "Debugging winner with sheep collected  ")
        (goto _label Break)))))