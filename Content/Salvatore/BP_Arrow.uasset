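; BP_Arrow is an objective pointer that hovers at an offset from its associated car and shows the direction of the current target.
; Each Tick it moves with the car, then points at the car's Barn if the car has a Sheep, otherwise at its SheepOnFarm.
; Look-at rotations are measured from the car with a 90-degree yaw correction; only the sheep target also applies pitch and roll.
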(event EventBeginPlay)

(event Collision|EventActorBeginOverlap
  (params (OtherActor :type Actor%20Object%20Reference)))

(event EventTick
  (params (DeltaSeconds :type Float%20%28single-precision%29))
  (bind _associatedcaractor (Variables|Default|GetAssociatedCarActor))
  (bind _associatedcaractor_2 (Variables|Default|GetAssociatedCarActor))
  (bind _associatedcaractor_3 (Variables|Default|GetAssociatedCarActor))
  (bind _returnvalue (Transformation|GetActorLocation _associatedcaractor_3))
  (bind _sheeponfarm (Variables|/Game/VehicleTemplate/Blueprints/OffroadCar/BP_OffroadCar_Pawn.BP_OffroadCar_Pawn_C|GetSheepOnFarm _associatedcaractor_2))
  (bind _returnvalue_2 (Transformation|GetActorTransform _sheeponfarm))
  (bind _returnvalue_3 (Math|Rotator|FindLookatRotation _returnvalue (.location _returnvalue_2)))
  (Utilities|IsValid _associatedcaractor
    (:Is%20Valid
      (Transformation|SetActorLocation (+ (Transformation|GetActorLocation _associatedcaractor) (Variables|Default|GetOffsetFromCarVector)) false false)
      (Utilities|IsValid (Variables|/Game/VehicleTemplate/Blueprints/OffroadCar/BP_OffroadCar_Pawn.BP_OffroadCar_Pawn_C|GetSheep _associatedcaractor)
        (:Is%20Valid
          (Transformation|SetActorRotation (Math|Rotator|MakeRotator 0.0 0.0 (+ (.yaw (Math|Rotator|FindLookatRotation (Transformation|GetActorLocation (Variables|Default|GetAssociatedCarActor)) (.location (Transformation|GetActorTransform (Variables|/Game/VehicleTemplate/Blueprints/OffroadCar/BP_OffroadCar_Pawn.BP_OffroadCar_Pawn_C|GetBarn (Variables|Default|GetAssociatedCarActor)))))) 9e+01))))
        (:Is%20Not%20Valid
          (Utilities|IsValid _sheeponfarm
            (:Is%20Valid
              (Transformation|SetActorRotation (Math|Rotator|MakeRotator (.roll _returnvalue_3) (.pitch _returnvalue_3) (+ (.yaw _returnvalue_3) 9e+01))))))))))

(fn ConstructionScript)