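; BP_Barn is the drop-off point where the player's offroad car delivers collected sheep.
; When the car overlaps its Box, it adds an audio component and calls SheepCollected on the pawn, printing a success or failure message.
; On success, SpawnSheep spawns a new BP_Sheep at random positive X/Y within MapRadius and assigns it to every car pawn's SheepOnFarm.
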(event OnComponentBeginOverlap(Box)
  (params (OverlappedComponent :type Primitive%20Component%20Object%20Reference) (OtherActor :type Actor%20Object%20Reference) (OtherComp :type Primitive%20Component%20Object%20Reference) (OtherBodyIndex :type Integer) (bFromSweep :type Boolean) (SweepResult :type Hit%20Result%20Structure%20%28by%20ref%29))
  (bind _asbp_offroad_car_pawn (Utilities|Casting|CastToBP_OffroadCar_Pawn OtherActor))
  (AddComponent|AddAudioComponent false)
  (bind _success (Default|SheepCollected _asbp_offroad_car_pawn))
  (if _success
    (Development|PrintString "Sheep is in safety!!!")
    (CallFunction|SpawnSheep)
    (else
      (Development|PrintString "Get some sheep already!!!"))))

(event EventBeginPlay)

(event Collision|EventActorBeginOverlap
  (params (OtherActor :type Actor%20Object%20Reference)))

(event EventTick
  (params (DeltaSeconds :type Float%20%28single-precision%29)))

(fn ConstructionScript)

(fn SpawnSheep
  (bind _mapradius (LocalVariables|GetMapRadius))
  (bind _returnvalue (Math|Conversions|ToFloat(Integer) _mapradius))
  (bind _returnvalue_2 (* _returnvalue 0.9))
  (bind _returnvalue_3 (Math|Float|Truncate _returnvalue_2))
  (bind _returnvalue_4 (Math|Random|RandomInteger _returnvalue_3))
  (bind _returnvalue_5 (Game|SpawnActorfromClass "/Game/Sheep/BP_Sheep.BP_Sheep_C" (Math|Transform|MakeTransform (Math|Vector|MakeVector (Math|Conversions|ToFloat(Integer) _returnvalue_4) (Math|Conversions|ToFloat(Integer) _returnvalue_4) 2.5e+02) "0, 0, 0" "1.000000,1.000000,1.000000") "Undefined" "MultiplyWithRoot" 0 0))
  (Development|PrintString (Utilities|String|ToString(Transform) (Transformation|GetActorTransform _returnvalue_5)))
  (bind _outactors (Actor|GetAllActorsOfClass "/Game/VehicleTemplate/Blueprints/OffroadCar/BP_OffroadCar_Pawn.BP_OffroadCar_Pawn_C"))
  (for _array_element _outactors
    (Variables|/Game/VehicleTemplate/Blueprints/OffroadCar/BP_OffroadCar_Pawn.BP_OffroadCar_Pawn_C|SetSheepOnFarm _array_element _returnvalue_5)))